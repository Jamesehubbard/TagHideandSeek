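; Player Blueprint for what appears to be a hide-and-seek game, with Enhanced Input movement and look controls.
; Movement follows the control rotation, and look input drives controller yaw and pitch.
; Non-seekers have their Cylinder component hidden in game while moving and shown again when movement input completes.
; The E key uses a FlipFlop to add and remove a HiddenScreen widget on the player's screen.
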(event Input|EnhancedActionEvents|EnhancedInputActionMove_IA
  (params (ActionValue :type Vector%202D%20Structure) (ElapsedSeconds :type Float%20%28double-precision%29) (TriggeredSeconds :type Float%20%28double-precision%29) (InputAction :type Input%20Action%20Object%20Reference :default "/Game/Input/Move_IA.Move_IA"))
  (bind _returnvalue (Pawn|GetControlRotation :!class /Script/Engine.Pawn))
  (:Triggered
    (Pawn|Input|AddMovementInput (Math|Vector|GetRightVector (Math|Rotator|MakeRotator (.roll _returnvalue) 0.0 (.yaw _returnvalue))) (.x ActionValue) false)
    (Pawn|Input|AddMovementInput (Math|Vector|GetForwardVector (Math|Rotator|MakeRotator 0.0 0.0 (.yaw (Pawn|GetControlRotation :!class /Script/Engine.Pawn)))) (.y ActionValue) false)
    (if (not (Variables|Default|GetIs%20Seeker))
      (Development|SetHiddeninGame (Variables|Default|GetCylinder) true false)))
  (:Completed
    (if (not (Variables|Default|GetIs%20Seeker))
      (Development|SetHiddeninGame (Variables|Default|GetCylinder) false false))))

(event Input|EnhancedActionEvents|EnhancedInputActionLook_IA
  (params (ActionValue :type Vector%202D%20Structure) (ElapsedSeconds :type Float%20%28double-precision%29) (TriggeredSeconds :type Float%20%28double-precision%29) (InputAction :type Input%20Action%20Object%20Reference :default "/Game/Input/Look_IA.Look_IA"))
  (Pawn|Input|AddControllerYawInput (.x ActionValue))
  (Pawn|Input|AddControllerPitchInput (.y ActionValue)))

(event Input|KeyboardEvents|E
  (params (Key :type Key%20Structure :default "None"))
  (:Pressed
    (Utilities|FlowControl|FlipFlop
      (:A
        (bind _returnvalue (UserInterface|CreateWidget "/Game/Widgets/HiddenScreen_WIdget.HiddenScreen_WIdget_C"))
        (UserInterface|Viewport|AddtoPlayerScreen _returnvalue))
      (:B
        (Widget|RemovefromParent _returnvalue)))))

(fn ConstructionScript)