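; Game mode that sets up local split-screen multiplayer with one seeker, spawning a player for each PlayerStart in the level.
; On BeginPlay it creates a local player per start, adds the THS_IMC input mapping, then spawns and possesses a Player_BP.
; The first player's pawn is flagged as the seeker.
; A parallel sequence branch briefly force-disables split screen after a short delay, then restores it.
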(event EventBeginPlay
  (Utilities|FlowControl|Sequence
    (:then_0
      (bind _outactors (Actor|GetAllActorsOfClass "/Script/Engine.PlayerStart"))
      (for (_array_element _array_index) _outactors
        (bind _output_get (Variables|Default|SetArray%20Index _array_index))
        (bind _returnvalue (Class|GameplayStatics|CreatePlayer _output_get))
        (if (> (Variables|Default|GetArray%20Index) 0)
          (Input|AddMappingContext (PlayerController|LocalPlayerSubsystems|GetEnhancedInputLocalPlayerSubsystem _returnvalue) "/Game/Input/THS_IMC.THS_IMC" 0 "(bIgnoreAllPressedKeysUntilRelease=True,bForceImmediately=False,bNotifyUserSettings=False)")
          (bind _returnvalue_2 (Game|SpawnActorfromClass "/Game/Blueprints/Player_BP.Player_BP_C" (Transformation|GetActorTransform _array_element) "Undefined" "MultiplyWithRoot" 0 0))
          (Pawn|Possess (Game|GetPlayerController (Variables|Default|GetArray%20Index)) _returnvalue_2)
          (else
            (Input|AddMappingContext (PlayerController|LocalPlayerSubsystems|GetEnhancedInputLocalPlayerSubsystem (Game|GetPlayerController 0)) "/Game/Input/THS_IMC.THS_IMC" 0 "(bIgnoreAllPressedKeysUntilRelease=True,bForceImmediately=False,bNotifyUserSettings=False)")
            (bind _returnvalue_3 (Game|SpawnActorfromClass "/Game/Blueprints/Player_BP.Player_BP_C" (Transformation|GetActorTransform _array_element) "Undefined" "MultiplyWithRoot" 0 0))
            (Pawn|Possess (Game|GetPlayerController 0) _returnvalue_3)
            (Variables|/Game/Blueprints/Player_BP.Player_BP_C|SetIs%20Seeker _returnvalue_3 true)))))
    (:then_1
      (Utilities|FlowControl|Delay 3.0)
      (Class|GameplayStatics|SetForceDisableSplitscreen true)
      (Utilities|FlowControl|Delay 2.0)
      (Class|GameplayStatics|SetForceDisableSplitscreen false))))

(fn ConstructionScript)